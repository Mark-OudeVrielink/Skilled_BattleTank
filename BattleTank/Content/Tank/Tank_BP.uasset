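; Player-controllable tank Blueprint that handles camera aiming, firing and track-driven movement.
; BeginPlay registers the Barrel and Turret components, and fire input calls Fire.
; Aim axes rotate an azimuth gimbal and spring arm separately for camera yaw and pitch.
; Each throttle axis applies its track's SetThrottle result as a force on the Body at that track's location, while LeftStick sends forward intent to TankMovementComponent.
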(event EventBeginPlay
  (Class|Tank|SetBarrel (Variables|Default|GetBarrel))
  (Class|Tank|SetTurret (Variables|Default|GetTurret)))

(event Input|ActionEvents|InputActionFireInput
  (params (Key :type Key%20Structure))
  ;[1 1 1] Tank firing
  (:Pressed
    (Class|Tank|Fire)))

(event Input|AxisEvents|InputAxisAimAzimuth
  (params (AxisValue :type Float%20%28single-precision%29))
  ;[1 1 1] Camera aim
  (Transformation|AddLocalRotation (Variables|Default|GetAzimuthGimbal) (Math|Rotator|MakeRotator 0.0 0.0 AxisValue) false false))

(event Input|AxisEvents|InputAxisLeftThrottle
  (params (AxisValue :type Float%20%28single-precision%29))
  (bind _left_track (Variables|Default|GetLeft%20Track))
  ;[1 1 1] Throttle
  (bind _returnvalue (Class|TankTrack|SetThrottle _left_track AxisValue))
  (Class|PrimitiveComponent|AddForceatLocation (Variables|Default|GetBody) _returnvalue (Transformation|GetWorldLocation _left_track) "None"))

(event Input|AxisEvents|InputAxisRightThrottle
  (params (AxisValue :type Float%20%28single-precision%29))
  (bind _right_track (Variables|Default|GetRight%20Track))
  ;[1 1 1] Throttle
  (bind _returnvalue (Class|TankTrack|SetThrottle _right_track AxisValue))
  (Class|PrimitiveComponent|AddForceatLocation (Variables|Default|GetBody) _returnvalue (Transformation|GetWorldLocation _right_track) "None"))

(event Input|AxisEvents|InputAxisAimElevation
  (params (AxisValue :type Float%20%28single-precision%29))
  ;[1 1 1] Camera aim
  (Transformation|AddLocalRotation (Variables|Default|GetSpringArm) (Math|Rotator|MakeRotator 0.0 AxisValue 0.0) false false))

(event Input|AxisEvents|InputAxisLeftStick
  (params (AxisValue :type Float%20%28single-precision%29))
  ;[1 1 1] Throttle
  (Class|TankMovementComponent|IntendMoveForward (Variables|Default|Get_tankMovementComponent) AxisValue))

(fn ConstructionScript)